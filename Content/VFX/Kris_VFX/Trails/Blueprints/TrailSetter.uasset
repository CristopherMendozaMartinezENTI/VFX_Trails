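; Anim notify state that starts and stops sword trail VFX over its window in an animation.
; On begin, it casts the mesh owner to DUMMY_BlueprintSword, begins trails on its particle system between the "VFX Start" and "VFX End" sockets, and spawns its scattering emitter attached at "VFX Center".
; On end, it only ends the trails; the spawned emitter is not explicitly stopped.
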(fn `Received_NotifyBegin`
  (params (MeshComp :type "SkeletalMeshComponent Object Reference") (Animation :type "AnimSequenceBase Object Reference") (TotalDuration :type "Float (double-precision)"))
  (returns (ReturnValue :type Boolean))
  (locals (NewLocalVar_0 :type "ParticleSystem Object Reference" :default "ParticleSystem'/Game/AttackTrailFX01/Particles/P_ky_attackTrail01.P_ky_attackTrail01'") (NewLocalVar_1 :type "ParticleSystemComponent Object Reference"))
  (bind _asdummy_blueprint_sword (cast `/Game/VFX/Kris_VFX/Trails/Blueprints/DUMMY_BlueprintSword` (`ActorComponent.GetOwner` MeshComp)))
  (`ParticleSystemComponent.BeginTrails` (`/Game/VFX/Kris_VFX/Trails/Blueprints/DUMMY_BlueprintSword.ParticleSystem` _asdummy_blueprint_sword) "VFX Start" "VFX End" "ETrailWidthMode_FromCentre" 1.0)
  (`GameplayStatics.SpawnEmitterAttached` (`/Game/VFX/Kris_VFX/Trails/Blueprints/DUMMY_BlueprintSword.Scattering VFX` _asdummy_blueprint_sword) MeshComp "VFX Center" (0.0 0.0 0.0) (struct) (1.0 1.0 1.0) "SnapToTarget")
  (return false))

(fn `Received_NotifyEnd`
  (params (MeshComp :type "SkeletalMeshComponent Object Reference") (Animation :type "AnimSequenceBase Object Reference"))
  (returns (ReturnValue :type Boolean))
  (bind _asdummy_blueprint_sword (cast `/Game/VFX/Kris_VFX/Trails/Blueprints/DUMMY_BlueprintSword` (`ActorComponent.GetOwner` MeshComp)))
  (`ParticleSystemComponent.EndTrails` (`/Game/VFX/Kris_VFX/Trails/Blueprints/DUMMY_BlueprintSword.ParticleSystem` _asdummy_blueprint_sword))
  (return false))