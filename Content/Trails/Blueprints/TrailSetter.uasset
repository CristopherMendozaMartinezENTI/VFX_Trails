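; TrailSetter is an animation notify state that drives trail effects on a DUMMY_Blueprint owner during an animation window.
; On begin, it starts trails on the owner's ParticleSystem between the "VFX Start" and "VFX End" sockets, then spawns the owner's ScatteringVFX emitter attached at "VFX Center".
; On end, it calls EndTrails but leaves the scattering emitter untouched.
; Any other owner type is ignored through the cast.
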(fn `Received_NotifyBegin`
  (params (MeshComp :type "SkeletalMeshComponent Object Reference") (Animation :type "AnimSequenceBase Object Reference") (TotalDuration :type "Float (double-precision)"))
  (returns (ReturnValue :type Boolean))
  (locals (NewLocalVar_0 :type "ParticleSystem Object Reference" :default "ParticleSystem'/Game/AttackTrailFX01/Particles/P_ky_attackTrail01.P_ky_attackTrail01'") (NewLocalVar_1 :type "ParticleSystemComponent Object Reference"))
  (bind _asdummy_blueprint (cast `/Game/Trails/Blueprints/DUMMY_Blueprint` (`ActorComponent.GetOwner` MeshComp)))
  (`ParticleSystemComponent.BeginTrails` (`/Game/Trails/Blueprints/DUMMY_Blueprint.ParticleSystem` _asdummy_blueprint) "VFX Start" "VFX End" "ETrailWidthMode_FromCentre" 1.0)
  (`GameplayStatics.SpawnEmitterAttached` (`/Game/Trails/Blueprints/DUMMY_Blueprint.Scattering VFX` _asdummy_blueprint) MeshComp "VFX Center" (0.0 0.0 0.0) (struct) (1.0 1.0 1.0) "SnapToTarget")
  (return false))

(fn `Received_NotifyEnd`
  (params (MeshComp :type "SkeletalMeshComponent Object Reference") (Animation :type "AnimSequenceBase Object Reference"))
  (returns (ReturnValue :type Boolean))
  (bind _asdummy_blueprint (cast `/Game/Trails/Blueprints/DUMMY_Blueprint` (`ActorComponent.GetOwner` MeshComp)))
  (`ParticleSystemComponent.EndTrails` (`/Game/Trails/Blueprints/DUMMY_Blueprint.ParticleSystem` _asdummy_blueprint))
  (return false))